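; Interactable single-door prop, named as unbreachable, whose Blueprint is a partial reconstruction that an author note calls unneeded.
; On a breached state with a valid BreachedMesh, OnStateChanged swaps the handle and door meshes for the breached one.
; If the state actually changed, it also spawns breach VFX on the handle and posts an audio event.
; The Timeline logic for handle primitive data and OnStateDone never runs, and the construction script is empty.
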(event `self.OnStateChanged`
  (params (OldState :type "ESBZGateState Enum" :default "OpenForward") (NewState :type "ESBZGateState Enum" :default "OpenForward") (bIsInitialStateChange :type Boolean))
  ;[1 1 1] You don't need any of these, I was just trying to reconstruct the BP but it is not needed.
  (if (or (`|EnumEquality` NewState "BreachedForward") (`|EnumEquality` NewState "BreachedBackward"))
    (if (`KismetSystemLibrary.IsValid` (`self.BreachedMesh`))
      (`|ExecutionSequence`
        (:`then_1`
          (`SceneComponent.SetVisibility` (`self.Hanlde_01`) false false)
          (`SceneComponent.SetVisibility` (`self.StaticDoorMesh`) false false)
          (`SceneComponent.SetVisibility` (`self.breached`) true false)
          (if (not (`|EnumEquality` OldState NewState))
            (`NiagaraFunctionLibrary.SpawnSystemAttached` (`self.BreachVFX`) (`self.Hanlde_01`) "None" (0.0 0.0 0.0) (struct :`Pitch` 90.0) "KeepRelativeOffset")
            (`AkGameplayStatics.PostEvent` null null 0 (delegate `Temp_delegate_Variable`) (`|MakeArray`) true))))
      (else
        (`|ExecutionSequence` :!label _label)))
    (else
      (goto _label))))

(event `Temp_delegate_Variable`
  (params (CallbackType :type "EAkCallbackType Enum" :default "EndOfEvent") (CallbackInfo :type "AkCallbackInfo Object Reference"))
  ;[1 1 1] You don't need any of these, I was just trying to reconstruct the BP but it is not needed.
)

(fn `UserConstructionScript`)